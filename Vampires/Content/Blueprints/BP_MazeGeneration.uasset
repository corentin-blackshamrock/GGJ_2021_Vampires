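; Procedural maze generator actor that builds a square tile grid on BeginPlay and spawns it as BP_Ground and BP_Wall actors.
; Ground fills the all-wall grid first, then weighted-random rooms are stamped at random non-overlapping spots and walls spawn on remaining wall tiles.
; ParseRoomCsvs converts data tables into equally weighted room templates, but nothing here calls it.
; Corridor generation is unfinished: it picks a start tile but never carves tiles.
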(event `self.ReceiveBeginPlay`
  (`self.InitializeCache`)
  (`self.GenerateMaze`))

(fn `GenerateCorridor`
  (locals (CorridorStartTile :type "IntPoint Structure") (CorridorEndTile :type "IntPoint Structure") (CorridorPath :type "Array of IntPoint Structure"))
  (set `local.CorridorStartTile` (`self.GetValidCorridorEdge`))
  (set `local.CorridorEndTile` (`local.CorridorEndTile`))
  (`KismetArrayLibrary.Array_Add` (`local.CorridorPath`)))

(fn `GenerateCorridors`
  (for _ (range (`self.CorridorCount`))
    (`self.GenerateCorridor`)))

(fn `GenerateLayer`
  (params (ZOffset :type "Float (double-precision)") (TileClass :type "Actor Class Reference"))
  (locals (Index :type Integer))
  (bind _index (`local.Index`))
  (while (< (`local.Index`) (`KismetArrayLibrary.Array_Length` (`self.Tiles`)))
    (if (not (`self.IsMazeTileEmpty` _index))
      (`|SpawnActorFromClass` (`local.TileClass`) (`KismetMathLibrary.MakeTransform` (`self.GetTilePosition` _index (`local.ZOffset`))) "AlwaysSpawn" "OverrideRootScale" null null))
    (`/Engine/EditorBlueprintResources/StandardMacros.IncrementInt` (`local.Index`))))

(fn `GenerateMaze`
  (`self.InitializeTiles`)
  (`self.GenerateLayer` (`self.GroundLayerZOffset`) "/Game/Blueprints/BP_Ground.BP_Ground_C")
  (`self.GenerateRooms`)
  (`self.GenerateCorridors`)
  (`self.GenerateLayer` (`self.WallLayerZOffset`) "/Game/Blueprints/BP_Wall.BP_Wall_C"))

(fn `GenerateRooms`
  (locals (RoomSelected :type "/Game/BlueprintTypes/MazeRoom Structure"))
  (for _ (range (`self.RoomCount`))
    (set `local.RoomSelected` (`self.GetRandomRoom`))
    (for _ (range (`self.MaxRoomIterations`))
      (bind _bplaced (`self.TryPlaceRoomAtRandomPosition` (`local.RoomSelected`)))
      (if _bplaced
        (break)))))

(fn `GetDownTileCoordinates`
  (params (TileCoords :type "IntPoint Structure"))
  (returns (DownTileCoords :type "IntPoint Structure"))
  (bind (_x _y) (break `IntPoint` TileCoords))
  (return (make `IntPoint` (- _x 1) _y)))

(fn `GetLeftTileCoordinates`
  (params (TileCoords :type "IntPoint Structure"))
  (returns (LeftTileCoords :type "IntPoint Structure"))
  (bind (_x _y) (break `IntPoint` TileCoords))
  (return (make `IntPoint` _x (- _y 1))))

(fn `GetMazeNeighbourTileTypes`
  (params (TileCoords :type "IntPoint Structure"))
  (returns (NeighboursTileType :type "/Game/BlueprintTypes/NeighboursTileType Structure"))
  (locals (UpTileType :type "/Game/BlueprintTypes/TileInfo Structure") (DownTileType :type "/Game/BlueprintTypes/TileInfo Structure") (LeftTileType :type "/Game/BlueprintTypes/TileInfo Structure") (RightTileType :type "/Game/BlueprintTypes/TileInfo Structure"))
  (bind _downtilecoords (`self.GetDownTileCoordinates` (`local.TileCoords`)))
  (bind _lefttilecoords (`self.GetLeftTileCoordinates` (`local.TileCoords`)))
  (bind _righttilecoords (`self.GetRightTileCoordinates` (`local.TileCoords`)))
  (bind _uptilecoords (`self.GetUpTileCoordinates` (`local.TileCoords`)))
  (bind _tileindex (`self.GetTileIndexWithPoint` _downtilecoords (`self.TileDimensionSize`)))
  (bind _tileindex_2 (`self.GetTileIndexWithPoint` _lefttilecoords (`self.TileDimensionSize`)))
  (bind _tileindex_3 (`self.GetTileIndexWithPoint` _righttilecoords (`self.TileDimensionSize`)))
  (bind _tileindex_4 (`self.GetTileIndexWithPoint` _uptilecoords (`self.TileDimensionSize`)))
  (`|ExecutionSequence`
    (:`then_0`
      (if (`self.IsMazeTileCoordsValid` _uptilecoords)
        (set `local.UpTileType` (make `/Game/BlueprintTypes/TileInfo` (`.Type_2_D07888534CDD6FF6D6AB5EAFE4CE161E` (break `/Game/BlueprintTypes/TileData` (`|GetArrayItem` (`self.Tiles`) _tileindex_4))) (`self.GetTilePosition` _tileindex_4 (`self.WallLayerZOffset`))))))
    (:`then_1`
      (if (`self.IsMazeTileCoordsValid` _downtilecoords)
        (set `local.DownTileType` (make `/Game/BlueprintTypes/TileInfo` (`.Type_2_D07888534CDD6FF6D6AB5EAFE4CE161E` (break `/Game/BlueprintTypes/TileData` (`|GetArrayItem` (`self.Tiles`) _tileindex))) (`self.GetTilePosition` _tileindex (`self.WallLayerZOffset`))))))
    (:`then_2`
      (if (`self.IsMazeTileCoordsValid` _lefttilecoords)
        (set `local.LeftTileType` (make `/Game/BlueprintTypes/TileInfo` (`.Type_2_D07888534CDD6FF6D6AB5EAFE4CE161E` (break `/Game/BlueprintTypes/TileData` (`|GetArrayItem` (`self.Tiles`) _tileindex_2))) (`self.GetTilePosition` _tileindex_2 (`self.WallLayerZOffset`))))))
    (:`then_3`
      (if (`self.IsMazeTileCoordsValid` _righttilecoords)
        (set `local.RightTileType` (make `/Game/BlueprintTypes/TileInfo` (`.Type_2_D07888534CDD6FF6D6AB5EAFE4CE161E` (break `/Game/BlueprintTypes/TileData` (`|GetArrayItem` (`self.Tiles`) _tileindex_3))) (`self.GetTilePosition` _tileindex_3 (`self.WallLayerZOffset`))))))
    (:`then_4`
      (return (make `/Game/BlueprintTypes/NeighboursTileType` (`local.UpTileType`) (`local.DownTileType`) (`local.LeftTileType`) (`local.RightTileType`))))))

(fn `GetMazeTileCoordinates`
  (params (Index :type Integer))
  (returns (X :type Integer) (Y :type Integer))
  (bind (_x _y) (`self.GetTileCoordinates` Index (`self.TileDimensionSize`)))
  (return _x _y))

(fn `GetRandomRoom`
  (returns (Room :type "/Game/BlueprintTypes/MazeRoom Structure"))
  (locals (Index :type Integer) (CurrentWeight :type "Float (double-precision)") (RandomWeight :type "Float (double-precision)"))
  (bind (_weight _room) (break `/Game/BlueprintTypes/WeightedRoom` (`|GetArrayItem` (`self.Rooms`) (`local.Index`))))
  (set `local.RandomWeight` (`KismetMathLibrary.RandomFloatInRange` 0.0 (`self.RoomsTotalWeight`)))
  (while (< (`local.Index`) (`KismetArrayLibrary.Array_Length` (`self.Rooms`)))
    (bind _output_get (set `local.CurrentWeight` (+ (`local.CurrentWeight`) _weight)))
    (if (>= _output_get (`local.RandomWeight`))
      (return _room)
      (else
        (`/Engine/EditorBlueprintResources/StandardMacros.IncrementInt` (`local.Index`))))))

(fn `GetRightTileCoordinates`
  (params (TileCoords :type "IntPoint Structure"))
  (returns (RightTileCoords :type "IntPoint Structure"))
  (bind (_x _y) (break `IntPoint` TileCoords))
  (return (make `IntPoint` _x (+ _y 1))))

(fn `GetTileCoordinates`
  (params (Index :type Integer) (RowSize :type Integer))
  (returns (X :type Integer) (Y :type Integer))
  (return (/ Index RowSize) (mod Index RowSize)))

(fn `GetTileCount`
  (returns (TileCount :type Integer))
  (return (* (`self.TileDimensionSize`) (`self.TileDimensionSize`))))

(fn `GetTileIndex`
  (params (X :type Integer) (Y :type Integer) (RowSize :type Integer))
  (returns (TileIndex :type Integer))
  (return (+ Y (* X RowSize))))

(fn `GetTileIndexWithPoint`
  (params (Point :type "IntPoint Structure") (RowSize :type Integer))
  (returns (TileIndex :type Integer))
  (bind (_x _y) (break `IntPoint` Point))
  (return (+ _y (* _x RowSize))))

(fn `GetTilePosition`
  (params (Index :type Integer) (ZOffset :type "Float (double-precision)"))
  (returns (TilePosition :type "Vector Structure"))
  (bind _tilesize (`self.TileSize`))
  (bind (_x _y) (`self.GetMazeTileCoordinates` (`local.Index`)))
  (return (+ (`self.K2_GetActorLocation`) (`KismetMathLibrary.MakeVector` (* _tilesize (`KismetMathLibrary.Conv_IntToDouble` _x)) (* _tilesize (`KismetMathLibrary.Conv_IntToDouble` _y)) (`local.ZOffset`)))))

(fn `GetUpTileCoordinates`
  (params (TileCoords :type "IntPoint Structure"))
  (returns (UpTileCoords :type "IntPoint Structure"))
  (bind (_x _y) (break `IntPoint` TileCoords))
  (return (make `IntPoint` (+ _x 1) _y)))

(fn `GetValidCorridorEdge`
  (returns (TileCoords :type "IntPoint Structure"))
  (locals (MaxIterationCount :type Integer :default 1000) (SelectedTileCoords :type "IntPoint Structure"))
  (bind _corridorstarttilerange (`self.CorridorStartTileRange`))
  (bind _corridorstarttilerange_2 (`self.CorridorStartTileRange`))
  (bind (_x _y) (break `IntPoint` (`local.SelectedTileCoords`)))
  (bind _returnvalue (`KismetMathLibrary.RandomIntegerInRange` (`self.CorridorEdgeOffsetFromBorder`) (- (- (`self.TileDimensionSize`) (`self.CorridorEdgeOffsetFromBorder`)) 1)))
  (for _ (range (`local.MaxIterationCount`))
    (set `local.SelectedTileCoords` (make `IntPoint` _returnvalue _returnvalue))
    (if (and (or (<= (- _x (`self.CorridorEdgeOffsetFromBorder`)) _corridorstarttilerange) (<= (- (- (`self.TileDimensionSize`) (`self.CorridorEdgeOffsetFromBorder`)) _x) _corridorstarttilerange)) (or (<= (- _y (`self.CorridorEdgeOffsetFromBorder`)) _corridorstarttilerange_2) (<= (- (- (`self.TileDimensionSize`) (`self.CorridorEdgeOffsetFromBorder`)) _y) _corridorstarttilerange_2)))
      (if (`|EnumInequality` (`.Type_2_D07888534CDD6FF6D6AB5EAFE4CE161E` (break `/Game/BlueprintTypes/TileData` (`|GetArrayItem` (`self.Tiles`) (`self.GetTileIndexWithPoint` (`local.SelectedTileCoords`))))) "NewEnumerator2")
        (return (`local.SelectedTileCoords`)))))
  (return (make `IntPoint` 1 1)))

(fn `InitializeCache`
  (`self.InitializeRoomTotalWeight`))

(fn `InitializeRoomTotalWeight`
  (locals (Index :type Integer))
  (while (< (`local.Index`) (`KismetArrayLibrary.Array_Length` (`self.Rooms`)))
    (set `self.RoomsTotalWeight` (+ (`self.RoomsTotalWeight`) (`.Weight_2_546C3BD24B0450BA7EC1E9857C5E67D1` (break `/Game/BlueprintTypes/WeightedRoom` (`|GetArrayItem` (`self.Rooms`) (`local.Index`))))))
    (`/Engine/EditorBlueprintResources/StandardMacros.IncrementInt` (`local.Index`))))

(fn `InitializeTiles`
  (locals (Index :type Integer))
  (while (< (`local.Index`) (`self.GetTileCount`))
    (`KismetArrayLibrary.Array_Add` (`self.Tiles`) (make `/Game/BlueprintTypes/TileData` "NewEnumerator1"))
    (`/Engine/EditorBlueprintResources/StandardMacros.IncrementInt` (`local.Index`))))

(fn `IsMazeTileCoordsValid`
  (params (TileCoords :type "IntPoint Structure"))
  (returns (bValid :type Boolean))
  (bind (_x _y) (break `IntPoint` TileCoords))
  (bind _tiledimensionsize (`self.TileDimensionSize`))
  (return (and (>= _x 0) (< _x _tiledimensionsize) (>= _y 0) (< _y _tiledimensionsize))))

(fn `IsMazeTileEmpty`
  (params (Index :type Integer))
  (returns (bEmpty :type Boolean))
  (return (`self.IsTileEmpty` (`self.Tiles`) Index)))

(fn `IsRoomMazeTile`
  (params (Index :type Integer))
  (returns (bRoom :type Boolean))
  (return (`|EnumEquality` (`.Type_2_D07888534CDD6FF6D6AB5EAFE4CE161E` (break `/Game/BlueprintTypes/TileData` (`|GetArrayItem` (`self.Tiles`) Index))) "NewEnumerator2")))

(fn `IsTileEmpty`
  (params (Tiles :type "Array of /Game/BlueprintTypes/TileData Structure") (Index :type Integer))
  (returns (bEmpty :type Boolean))
  (switch `/Game/BlueprintTypes/TileType` (`.Type_2_D07888534CDD6FF6D6AB5EAFE4CE161E` (break `/Game/BlueprintTypes/TileData` (`|GetArrayItem` Tiles Index)))
    (:`NewEnumerator1`
      (return false))
    (:`NewEnumerator0`
      _)
    (:`NewEnumerator2`
      _))
  (return true))

(fn `ParseRoomCsv`
  (params (RoomDataTable :type "DataTable Object Reference"))
  (returns (Room :type "/Game/BlueprintTypes/MazeRoom Structure"))
  (locals (TilesCsv :type "Array of String") (RowIndex :type Integer) (ColumnIndex :type Integer) (RoomWidth :type Integer) (RoomHeight :type Integer) (RoomTiles :type "Array of /Game/BlueprintTypes/TileData Structure"))
  (bind _roomdatatable (`local.RoomDataTable`))
  (`|ExecutionSequence`
    (:`then_0`
      (bind _outrownames (`DataTableFunctionLibrary.GetDataTableRowNames` _roomdatatable))
      (for _array_element _outrownames
        (bind _returnvalue (`|GetDataTableRow` _roomdatatable _array_element)
          (:`then`
            (bind (_c0 _c1 _c2 _c3 _c4 _c5 _c6 _c7 _c8 _c9) (break `/Game/BlueprintTypes/RoomCsv` _returnvalue))
            (for _array_element_2 (`|MakeArray` _c0 _c1 _c2 _c3 _c4 _c5 _c6 _c7 _c8 _c9)
              (`KismetArrayLibrary.Array_Add` (`local.TilesCsv`) _array_element_2))))))
    (:`then_1`
      (bind _width (`self.ParseRoomWidth` (`local.TilesCsv`)))
      (set `local.RoomWidth` _width)
      (bind _height (`self.ParseRoomHeight` (`local.TilesCsv`)))
      (set `local.RoomHeight` _height))
    (:`then_2`
      (set `local.RowIndex` (- (`local.RoomHeight`) 1))
      (while (>= (`local.RowIndex`) 0)
        (set `local.ColumnIndex` 0)
        (while (< (`local.ColumnIndex`) (`local.RoomWidth`))
          (switch `string` (`|GetArrayItem` (`local.TilesCsv`) (`self.GetTileIndex` (`local.RowIndex`) (`local.ColumnIndex`) 10))
            (:`X`
              (`KismetArrayLibrary.Array_Add` (`local.RoomTiles`) (make `/Game/BlueprintTypes/TileData` (enumliteral `/Game/BlueprintTypes/TileType` "NewEnumerator1"))))
            (:`O`
              (`KismetArrayLibrary.Array_Add` (`local.RoomTiles`) (make `/Game/BlueprintTypes/TileData` (enumliteral `/Game/BlueprintTypes/TileType` "NewEnumerator2")))))
          (`/Engine/EditorBlueprintResources/StandardMacros.IncrementInt` (`local.ColumnIndex`)))
        (`/Engine/EditorBlueprintResources/StandardMacros.DecrementInt` (`local.RowIndex`))))
    (:`then_3`
      (return (make `/Game/BlueprintTypes/MazeRoom` (`local.RoomWidth`) (`local.RoomHeight`) (`local.RoomTiles`))))))

(fn `ParseRoomCsvs`
  (`KismetArrayLibrary.Array_Clear` (`self.Rooms`))
  (for _array_element (`self.RoomCsvs`)
    (bind _room (`self.ParseRoomCsv` _array_element))
    (`KismetArrayLibrary.Array_Add` (`self.Rooms`) (make `/Game/BlueprintTypes/WeightedRoom` 1.0 _room))))

(fn `ParseRoomHeight`
  (params (TilesCsv :type "Array of String") (RowLength :type Integer :default 10))
  (returns (Height :type Integer))
  (locals (Index :type Integer))
  (bind _returnvalue (`KismetArrayLibrary.Array_Length` TilesCsv))
  (while (< (`local.Index`) _returnvalue)
    (if (`KismetStringLibrary.EqualEqual_StrStr` (`|GetArrayItem` (`local.TilesCsv`) (`local.Index`)) "-")
      (return (/ (`local.Index`) (`local.RowLength`)))
      (else
        (set `local.Index` (+ (`local.Index`) (`local.RowLength`))))))
  (return (/ _returnvalue (`local.RowLength`))))

(fn `ParseRoomWidth`
  (params (TilesCsv :type "Array of String") (MaxWidth :type Integer :default 10))
  (returns (Width :type Integer))
  (locals (Index :type Integer))
  (while (< (`local.Index`) MaxWidth)
    (if (`KismetStringLibrary.EqualEqual_StrStr` (`|GetArrayItem` (`local.TilesCsv`) (`local.Index`)) "-")
      (return (`local.Index`))
      (else
        (`/Engine/EditorBlueprintResources/StandardMacros.IncrementInt` (`local.Index`)))))
  (return MaxWidth))

(fn `SelectCorridorEndTile`
  (params (CorridorStartTile :type "IntPoint Structure"))
  (returns (CorridorEndTile :type "IntPoint Structure"))
  (locals (EndTileSelected :type "IntPoint Structure") (MaxIterationCount :type Integer :default 1000))
  (for _ (range (`local.MaxIterationCount`))
    (bind _output_get (set `local.EndTileSelected` (`self.GetValidCorridorEdge`)))
    (if (>= (`self.TileDistance` _output_get (`local.CorridorStartTile`)) (`self.MinCorridorLength`))
      (return (`local.EndTileSelected`))))
  (return (make `IntPoint` 1 1)))

(fn `TileDistance`
  (params (TileA :type "IntPoint Structure") (TileB :type "IntPoint Structure"))
  (returns (Distance :type Integer))
  (bind (_x _y) (break `IntPoint` (- TileA TileB)))
  (return (+ (`KismetMathLibrary.Abs_Int` _x) (`KismetMathLibrary.Abs_Int` _y))))

(fn `TryPlaceRoomAtRandomPosition`
  (params (Room :type "/Game/BlueprintTypes/MazeRoom Structure"))
  (returns (bPlaced :type Boolean))
  (locals (OriginRoomX :type Integer) (OriginRoomY :type Integer) (RoomX :type Integer) (RoomY :type Integer))
  (bind (_width _height) (break `/Game/BlueprintTypes/MazeRoom` (`local.Room`)))
  (bind (_width_2 _height_2 _tiles) (break `/Game/BlueprintTypes/MazeRoom` (`local.Room`)))
  (bind (_width_3 _height_3) (break `/Game/BlueprintTypes/MazeRoom` (`local.Room`)))
  (set `local.OriginRoomY` (+ (`KismetMathLibrary.RandomInteger` (- (- (`self.TileDimensionSize`) _width) 2)) 1))
  (set `local.OriginRoomX` (+ (`KismetMathLibrary.RandomInteger` (- (- (`self.TileDimensionSize`) _height) 2)) 1))
  (`|ExecutionSequence`
    (:`then_0`
      (for _index (range _height_3)
        (set `local.RoomX` _index)
        (for _index_2 (range _width_3)
          (set `local.RoomY` _index_2)
          (if (`self.IsRoomMazeTile` (`self.GetTileIndex` (+ (`local.OriginRoomX`) (`local.RoomX`)) (+ (`local.OriginRoomY`) (`local.RoomY`)) (`self.TileDimensionSize`)))
            (return false)))))
    (:`then_1`
      (for _index_3 (range _height_2)
        (set `local.RoomX` _index_3)
        (for _index_4 (range _width_2)
          (set `local.RoomY` _index_4)
          (`KismetArrayLibrary.Array_Set` (`self.Tiles`) (`self.GetTileIndex` (+ (`local.OriginRoomX`) (`local.RoomX`)) (+ (`local.OriginRoomY`) (`local.RoomY`)) (`self.TileDimensionSize`)) (`|GetArrayItem` _tiles (`self.GetTileIndex` (`local.RoomX`) (`local.RoomY`) _width_2))))))
    (:`then_2`
      (return true))))

(fn `UserConstructionScript`)