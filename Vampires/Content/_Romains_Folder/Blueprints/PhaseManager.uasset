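; Phase manager for the maze game, running timed first, pause and second phases before an end state.
; Initialize links the maze to RomainsTopDownController and teleports the player to a random walkable tile.
; Once initialized, Tick advances phase timers with camera fades and debug prints.
; The second phase ends on timeout or death with the same result; the other result's branch is hard-coded false, and the end screen only prints.
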(event `self.ReceiveTick`
  (params (DeltaSeconds :type "Float (single-precision)"))
  (bind _playercameramanager (`PlayerController.PlayerCameraManager` (`GameplayStatics.GetPlayerController` 0)))
  (set `self.DeltaSeconds` DeltaSeconds)
  (`KismetSystemLibrary.PrintString` (`|GetEnumeratorNameAsString` (`self.GamePhase`)) true true (struct :`A` 1.0) 0.0)
  (if (`self.Initialized`)
    (switch `/Game/_Romains_Folder/Blueprints/EGamePhase` (`self.GamePhase`)
      (:`NewEnumerator2`
        (set `self.GamePhase` "NewEnumerator0"))
      (:`NewEnumerator0`
        (`KismetSystemLibrary.PrintString` (`KismetStringLibrary.Concat_StrStr` "Time remaning for fisrt phase :" (`KismetStringLibrary.Conv_DoubleToString` (- (`self.FirstPhaseTimeAmount`) (`self.TimerFirstPhase`)))) true true (struct :`G` 0.78412 :`B` 1.0 :`A` 1.0) 0.0)
        (bind _output_get (set `self.TimerFirstPhase` (+ (`self.TimerFirstPhase`) (`self.DeltaSeconds`))))
        (if (>= _output_get (`self.FirstPhaseTimeAmount`))
          (set `self.GamePhase` "NewEnumerator4")
          (set `self.TimerFirstPhase` 0.0)
          (`PlayerCameraManager.StartCameraFade` :`self` _playercameramanager :`ToAlpha` 1.0 :`Duration` 2.0 :`bHoldWhenFinished` true)))
      (:`NewEnumerator4`
        (`KismetSystemLibrary.PrintString` (`KismetStringLibrary.Concat_StrStr` "Time remaning for pause :  " (`KismetStringLibrary.Conv_DoubleToString` (- (`self.PauseTimeAmount`) (`self.TimerPause`)))) true true (struct :`G` 0.876899 :`B` 1.0 :`A` 1.0) 0.0)
        (bind _output_get_2 (set `self.TimerPause` (+ (`self.TimerPause`) (`self.DeltaSeconds`))))
        (if (and (>= _output_get_2 2.5) (not (`self.alreadyFadeOut`)))
          (`PlayerCameraManager.StartCameraFade` :`self` _playercameramanager :`FromAlpha` 1.0 :`Duration` 2.5)
          (set `self.alreadyFadeOut` true))
        (if (>= _output_get_2 (`self.PauseTimeAmount`))
          (set `self.GamePhase` "NewEnumerator1")
          (set `self.TimerPause` 0.0)))
      (:`NewEnumerator1`
        (`KismetSystemLibrary.PrintString` (`KismetStringLibrary.Concat_StrStr` "Time remaning for second phase :  " (`KismetStringLibrary.Conv_DoubleToString` (- (`self.SecondPhaseTimeAmount`) (`self.TimerSecondPhase`)))) true true (struct :`G` 0.889458 :`B` 1.0 :`A` 1.0) 0.0)
        (bind _output_get_3 (set `self.TimerSecondPhase` (+ (`self.TimerSecondPhase`) (`self.DeltaSeconds`))))
        (if (>= _output_get_3 (`self.SecondPhaseTimeAmount`))
          (set `self.GameResult` "NewEnumerator1")
          (set `self.GamePhase` "NewEnumerator3" :!label _label)
          (set `self.TimerSecondPhase` 0.0)
          (`PlayerCameraManager.StartCameraFade` :`self` (`PlayerController.PlayerCameraManager` (`GameplayStatics.GetPlayerController` 0)) :`ToAlpha` 1.0 :`Duration` 1.5 :`bHoldWhenFinished` true)
          (elif false
            (set `self.GameResult` "NewEnumerator0")
            (goto _label)
            (elif (`/Game/_Romains_Folder/Blueprints/RomainsTopDownController.dead` (`self.Controller`))
              (set `self.GameResult` "NewEnumerator1")
              (goto _label)))))
      (:`NewEnumerator3`
        ;[1 1 1] AFFICHER ECRAN DE FIN
        (`KismetSystemLibrary.PrintString` (`|GetEnumeratorNameAsString` (`self.GameResult`)) true true (struct :`A` 1.0) 0.0)))))

(fn `Initialize`
  (locals (index :type Integer) (tempCoord :type "IntPoint Structure") (tempIndex :type Integer) (tempLocation :type "Vector Structure"))
  (bind _maze (`self.Maze`))
  (bind _maze_2 (`self.Maze`))
  (bind (_x _y) (`/Game/Blueprints/BP_MazeGeneration.GetMazeTileCoordinates` (`self.Maze`) (`local.tempIndex`)))
  (bind (_x_2 _y_2) (`/Game/Blueprints/BP_MazeGeneration.GetMazeTileCoordinates` (`self.Maze`) (`local.tempIndex`)))
  (bind (_tileposition_x _tileposition_y _tileposition_z) (`KismetMathLibrary.BreakVector` (`/Game/Blueprints/BP_MazeGeneration.GetTilePosition` _maze_2 (`/Game/Blueprints/BP_MazeGeneration.GetTileIndexWithPoint` _maze_2 (make `IntPoint` _x_2 _y_2) (`/Game/Blueprints/BP_MazeGeneration.TileDimensionSize` _maze_2)) 0.0)))
  (`|ExecutionSequence`
    (:`then_0`
      (bind _outactors (`GameplayStatics.GetAllActorsOfClass` "/Game/Blueprints/BP_MazeGeneration.BP_MazeGeneration_C"))
      (if (> (`KismetArrayLibrary.Array_Length` _outactors) 0)
        (set `self.Maze` (`|GetArrayItem` _outactors))))
    (:`then_1`
      (bind _outactors_2 (`GameplayStatics.GetAllActorsOfClass` "/Game/_Romains_Folder/Blueprints/RomainsTopDownController.RomainsTopDownController_C"))
      (if (> (`KismetArrayLibrary.Array_Length` _outactors_2) 0)
        (bind _output_get (set `self.Controller` (`|GetArrayItem` _outactors_2)))
        (set `/Game/_Romains_Folder/Blueprints/RomainsTopDownController.Maze` (`self.Maze`) _output_get)))
    (:`then_2`
      (while (not (`self.foundStartTile`))
        (bind _output_get_2 (set `local.tempIndex` (`KismetMathLibrary.RandomInteger` (`/Game/Blueprints/BP_MazeGeneration.GetTileCount` _maze))))
        (bind (_x_3 _y_3) (`/Game/Blueprints/BP_MazeGeneration.GetMazeTileCoordinates` _maze _output_get_2))
        (if (`/Game/Blueprints/BP_MazeGeneration.IsMazeTileWalkable` _maze (make `IntPoint` _x_3 _y_3))
          (set `self.foundStartTile` true)
          (set `local.tempLocation` (`KismetMathLibrary.MakeVector` (+ _tileposition_x 50.0) (+ _tileposition_y 50.0) (+ _tileposition_z 150.0)))
          (`self.K2_SetActorLocation` (`GameplayStatics.GetPlayerCharacter` 0) (`local.tempLocation`) false false)
          (`/Game/_Romains_Folder/Blueprints/RomainsTopDownController.SetTiles` (`self.Controller`) (make `IntPoint` _y _x))
          (set `/Game/_Romains_Folder/Blueprints/RomainsTopDownController.TempIndex` (`local.tempIndex`) (`self.Controller`))))
      (set `self.Initialized` true))))

(fn `UserConstructionScript`)